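; Actor Blueprint that animates what appears to be a small planetary display by continuously spinning itself and several named components.
; Each Tick adds yaw to the actor and local rotations to Planeta1, Planeta2, PlanetaExquisito and Ponto2, with Planeta2 alone turning on roll.
; Variables set most spin amounts, while Ponto2 uses a fixed negative yaw.
; Steps ignore delta time, so speeds depend on frame rate.
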(event EventBeginPlay)

(event Collision|EventActorBeginOverlap
  (params (OtherActor :type Actor%20Object%20Reference)))

(event EventTick
  (params (DeltaSeconds :type Float%20%28single-precision%29))
  (Transformation|AddActorLocalRotation (Math|Rotator|MakeRotator 0.0 0.0 (Variables|Default|GetRotator)) false false)
  (Transformation|AddLocalRotation (Variables|Default|GetPlaneta_1) (Math|Rotator|MakeRotator 0.0 0.0 (Variables|Default|Getrotate%202)) false false)
  (Transformation|AddLocalRotation (Variables|Default|GetPlaneta_2) (Math|Rotator|MakeRotator (Variables|Default|Getrotate%203) 0.0 0.0) false false)
  (Transformation|AddLocalRotation (Variables|Default|GetPlaneta_Exquisito) (Math|Rotator|MakeRotator 0.0 0.0 (Variables|Default|Getrotate%204)) false false)
  (Transformation|AddLocalRotation (Variables|Default|GetPonto_2) (Math|Rotator|MakeRotator 0.0 0.0 -3.0) false false))

(fn ConstructionScript)